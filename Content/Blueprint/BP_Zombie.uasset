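; BP_Zombie is an AI-driven zombie pawn that chases the player and can take damage.
; It starts an AI move toward the player on BeginPlay and reissues it each time the move succeeds.
; Any damage lowers Life and spawns a pooled Niagara hit effect.
; At zero Life or below it stops AI movement and plays a collapse sound, without destroying the actor.
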(event Custom|Chase%20Player
  (AI|AIMoveTo self "0, 0, 0" (Game|GetPlayerCharacter 0) 5.0 false
    (:OnSuccess
      (CallFunction|ChasePlayer))))

(event EventBeginPlay
  (CallFunction|ChasePlayer))

(event Game|Damage|EventAnyDamage
  (params (Damage :type Float%20%28single-precision%29) (DamageType :type Damage%20Type%20Object%20Reference) (InstigatedBy :type Controller%20Object%20Reference) (DamageCauser :type Actor%20Object%20Reference))
  (Variables|Default|Setlife (- (Variables|Default|Getlife) Damage))
  (Niagara|SpawnSystematLocation "/Game/Blueprint/NS_Damage.NS_Damage" (Transformation|GetActorLocation) "0, 0, 0" "1.000000,1.000000,1.000000" true true "AutoRelease")
  (if (<= (Variables|Default|Getlife) 0.0)
    (AI|Navigation|StopMovement (AI|GetAIController self))
    (Audio|PlaySoundatLocation "/Game/StarterContent/Audio/Collapse01.Collapse01" (Transformation|GetWorldLocation (Variables|Character|GetMesh)) "0, 0, 0" 1.0 1.0 0.0 0 0 0 0)))

(fn ConstructionScript)